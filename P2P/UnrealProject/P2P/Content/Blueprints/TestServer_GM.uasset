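; TestServer_GM, apparently a test game mode, runs a lobby server behind an on-screen test UI.
; On BeginPlay it constructs a LobbyServer object, passes it to a TestUI widget and shows that widget with UI-only input and a visible mouse cursor.
; The server object is advanced manually by forwarding each Tick to it.
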(event `self.ReceiveBeginPlay`
  (bind _returnvalue (`GameplayStatics.GetPlayerController` 0))
  (bind _returnvalue_2 (`|GenericCreateObject` "/Script/LobbyServer.LobbyServer"))
  (bind _output_get (set `self.Server` _returnvalue_2))
  (bind _returnvalue_3 (`|CreateWidget` "/Game/Blueprints/TestUI.TestUI_C"))
  (`/Game/Blueprints/TestUI.SetServer` _returnvalue_3 _output_get)
  (`UserWidget.AddToViewport` _returnvalue_3 0)
  (`WidgetBlueprintLibrary.SetInputMode_UIOnlyEx` _returnvalue _returnvalue_3)
  (set `PlayerController.bShowMouseCursor` true _returnvalue))

(event `self.ReceiveTick`
  (params (DeltaSeconds :type "Float (single-precision)"))
  (`LobbyServer.Tick` (`self.Server`)))

(fn `UserConstructionScript`)